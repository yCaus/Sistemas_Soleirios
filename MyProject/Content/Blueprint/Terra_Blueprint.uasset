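; Earth-like Actor (Terra) that spins around its local vertical axis every frame.
; Tick calls Rotation, which adds a yaw of delta seconds plus Velocity scaled by 360/86400 (degrees per day-second), so delta time is added rather than multiplied.
; Tick also sets location from an unfinished sine/cosine orbit with constant inputs, pinning the actor to the world origin.
; Translate and Distance logic is disconnected, and NewFunction is empty.
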(event EventBeginPlay)

(event Collision|EventActorBeginOverlap
  (params (OtherActor :type Actor%20Object%20Reference)))

(event EventTick
  (params (DeltaSeconds :type Float%20%28single-precision%29))
  (Utilities|FlowControl|Sequence
    (:then_0
      (|Rotation DeltaSeconds))
    (:then_1
      (Transformation|SetActorLocation (Math|Vector|MakeVector (* (Math|Trig|Sin(Radians) 0.0) 2e+04) (* (Math|Trig|Cos(Radians) 0.0) 0.0) 0.0) false false))))

(fn ConstructionScript)

(fn NewFunction)